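; A ventilation door that toggles between open and closed when its DoAction event fires.
; DoAction ignores calls while the OpenCloseTL timeline plays, otherwise running it forward or in reverse based on IsOpened.
; The timeline's OpenProgress track slides the door component's relative location between CloseLoc and OpenLoc without sweeping, and IsOpened flips when it finishes.
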(event `self.DoAction`
  (params (Caller :type "Actor Object Reference"))
  (if (`TimelineComponent.IsPlaying` (`self.OpenCloseTL`))
    _
    (elif (`self.IsOpened`)
      (bind (_direction _openprogress) (`Timeline|OpenCloseTL` :!via `ReverseFromEnd` :!label _label)
        (:`Update`
          (`SceneComponent.K2_SetRelativeLocation` (`self.VentilationDoor`) (`KismetMathLibrary.VLerp` (`self.CloseLoc`) (`self.OpenLoc`) _openprogress) false false))
        (:`Finished`
          (set `self.IsOpened` (not (`self.IsOpened`)))))
      (else
        (goto _label :!via `PlayFromStart`)))))

(fn `UserConstructionScript`)