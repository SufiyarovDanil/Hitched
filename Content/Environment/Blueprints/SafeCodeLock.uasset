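; SafeCodeLock is a single rotating code dial for a safe, cycling through six positions.
; DoAction, ignored while RotateTL plays, plays a button sound, advances CurrentNumber with wraparound, and starts the timeline.
; The timeline lerps the dial's relative yaw along the shortest path to a multiple of DeltaRot, then stores the final rotation.
; GetCurrentNumber exposes the position as a one-based value.
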(event `self.DoAction`
  (params (Caller :type "Actor Object Reference"))
  (bind (_currentrotation_roll _currentrotation_pitch _currentrotation_yaw) (`KismetMathLibrary.BreakRotator` (`self.CurrentRotation`)))
  (if (not (`TimelineComponent.IsPlaying` (`self.RotateTL`)))
    (`GameplayStatics.SpawnSoundAttached` "/Game/Sounds/Interact/button.button" (`self.Safe_Codelock`) "None" (0.0 0.0 0.0) (struct) "KeepRelativeOffset" false 0.3 1.0 0.0 null null)
    (bind _output_get (set `self.CurrentNumber` (mod (+ (`self.CurrentNumber`) 1) 6)))
    (bind (_direction _progress) (`Timeline|RotateTL` :!via `PlayFromStart`)
      (:`Update`
        (bind _returnvalue (`KismetMathLibrary.RLerp` (`KismetMathLibrary.MakeRotator` _currentrotation_roll _currentrotation_pitch _currentrotation_yaw) (`KismetMathLibrary.MakeRotator` _currentrotation_roll _currentrotation_pitch (* (`self.DeltaRot`) (`KismetMathLibrary.Conv_IntToDouble` _output_get))) _progress true))
        (`SceneComponent.K2_SetRelativeRotation` (`self.Safe_Codelock`) _returnvalue false false))
      (:`Finished`
        (set `self.CurrentRotation` _returnvalue)))))

(fn `GetCurrentNumber`
  (returns (Number :type Integer))
  (return (+ (`self.CurrentNumber`) 1)))

(fn `UserConstructionScript`)