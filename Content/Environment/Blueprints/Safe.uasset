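; Safe is an interactable Blueprint with a door that opens only when three code-lock dials show the right numbers.
; On BeginPlay it reads the three correct numbers from the questions of a child Letter actor.
; DoAction compares them with three SafeCodeLock child actors and, if all match, toggles the door open or closed.
; A timeline lerps the door rotation and blocks new actions while playing.
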(event `self.ReceiveBeginPlay`
  (bind _asletter (cast `/Game/Environment/Blueprints/Letter` (`ChildActorComponent.ChildActor` (`self.Letter`))))
  (for (_array_element _array_index) (`/Game/Environment/Blueprints/Letter.Questions` _asletter)
    (switch `int` _array_index
      (:`0`
        (set `self.RightNumber1` (`.RightAnswerNumber_11_A223527747A1EA256453ABAED679E029` (break `/Game/Petroleum/PetroleumQuiz` _array_element))))
      (:`1`
        (set `self.RighNumber2` (`.RightAnswerNumber_11_A223527747A1EA256453ABAED679E029` (break `/Game/Petroleum/PetroleumQuiz` _array_element))))
      (:`2`
        (set `self.RightNumber3` (`.RightAnswerNumber_11_A223527747A1EA256453ABAED679E029` (break `/Game/Petroleum/PetroleumQuiz` _array_element)))))))

(event `self.DoAction`
  (params (Caller :type "Actor Object Reference"))
  (if (not (`TimelineComponent.IsPlaying` (`self.OpenCloseTL`)))
    (bind _assafe_code_lock (cast `/Game/Environment/Blueprints/SafeCodeLock` (`ChildActorComponent.ChildActor` (`self.SafeCodeLock`))))
    (bind _assafe_code_lock_2 (cast `/Game/Environment/Blueprints/SafeCodeLock` (`ChildActorComponent.ChildActor` (`self.SafeCodeLock1`))))
    (bind _assafe_code_lock_3 (cast `/Game/Environment/Blueprints/SafeCodeLock` (`ChildActorComponent.ChildActor` (`self.SafeCodeLock2`))))
    (if (and (== (`/Game/Environment/Blueprints/SafeCodeLock.GetCurrentNumber` _assafe_code_lock) (`self.RightNumber1`)) (== (`/Game/Environment/Blueprints/SafeCodeLock.GetCurrentNumber` _assafe_code_lock_2) (`self.RighNumber2`)) (== (`/Game/Environment/Blueprints/SafeCodeLock.GetCurrentNumber` _assafe_code_lock_3) (`self.RightNumber3`)))
      (if (`self.IsOpened`)
        (bind (_direction _progress) (`Timeline|OpenCloseTL` :!via `ReverseFromEnd` :!label _label)
          (:`Update`
            (`SceneComponent.K2_SetRelativeRotation` (`self.Safe_Door`) (`KismetMathLibrary.RLerp` (`self.CloseRot`) (`self.OpenRot`) _progress true) false false))
          (:`Finished`
            (set `self.IsOpened` (not (`self.IsOpened`)))))
        (else
          (goto _label :!via `PlayFromStart`))))))

(fn `UserConstructionScript`)