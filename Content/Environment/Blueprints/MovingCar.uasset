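; MovingCar is an environment actor for a car that drives in a straight line and removes itself after a set time.
; Each Tick moves it along its forward vector by CarSpeed scaled by delta time, without sweep, so it does not check for collisions along the way.
; On BeginPlay it waits for LifeTime seconds and then destroys itself.
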(event `self.ReceiveBeginPlay`
  (`KismetSystemLibrary.Delay` (`self.LifeTime`))
  (`self.K2_DestroyActor`))

(event `self.ReceiveTick`
  (params (DeltaSeconds :type "Float (single-precision)"))
  (`self.K2_SetActorLocation` (+ (* (`self.GetActorForwardVector`) (* DeltaSeconds (`self.CarSpeed`))) (`self.K2_GetActorLocation`))))

(fn `UserConstructionScript`)