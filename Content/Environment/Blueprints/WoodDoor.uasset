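; Wooden door that toggles between open and closed when DoAction is called, ignoring calls while it is moving.
; A timeline plays forward or in reverse, lerping the Door component between closed and open rotations along the shortest path.
; IsInward overrides the open rotation at BeginPlay.
; Attached sounds play as each swing starts and when closing completes, and IsOpened flips when the timeline finishes.
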(event `self.ReceiveBeginPlay`
  (if (`self.IsInward`)
    (set `self.OpenStateRotation` (struct :`Yaw` -90.0))))

(event `self.DoAction`
  (params (Caller :type "Actor Object Reference"))
  (bind _door (`self.Door`))
  (bind _isopened (`self.IsOpened`))
  (if (`TimelineComponent.IsPlaying` (`self.DoorAnimTL`))
    _
    (elif (`self.IsOpened`)
      (`GameplayStatics.SpawnSoundAttached` "/Game/Sounds/Interact/doorws1.doorws1" _door "None" (0.0 0.0 0.0) (struct) "KeepRelativeOffset" false 1.0 1.0 0.0 null null)
      (bind (_direction _progress) (`Timeline|DoorAnimTL` :!via `Reverse` :!label _label)
        (:`Update`
          (`SceneComponent.K2_SetRelativeRotation` (`self.Door`) (`KismetMathLibrary.RLerp` (`self.CloseStateRotation`) (`self.OpenStateRotation`) _progress true) false false))
        (:`Finished`
          (if _isopened
            (`GameplayStatics.SpawnSoundAttached` "/Game/Sounds/Interact/doorw1c.doorw1c" (`self.Door`) "None" (0.0 0.0 0.0) (struct) "KeepRelativeOffset" false 1.0 1.0 0.0 null null))
          (set `self.IsOpened` (not _isopened))))
      (else
        (`GameplayStatics.SpawnSoundAttached` "/Game/Sounds/Interact/doorw1o.doorw1o" _door "None" (0.0 0.0 0.0) (struct) "KeepRelativeOffset" false 1.0 1.0 0.0 null null)
        (goto _label)))))

(fn `UserConstructionScript`)