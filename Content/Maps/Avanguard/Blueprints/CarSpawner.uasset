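; CarSpawner is an actor in the Avanguard map that repeatedly spawns MovingCar actors at its own transform.
; Tick accumulates elapsed time and, once it reaches the current period, spawns a car regardless of collisions.
; It then resets the timer and picks a new random interval of a few seconds, so traffic arrives at irregular gaps.
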(event `self.ReceiveTick`
  (params (DeltaSeconds :type "Float (single-precision)"))
  (set `self.TimeProgress` (+ (`self.TimeProgress`) DeltaSeconds))
  (if (>= (`self.TimeProgress`) (`self.TimePeriod`))
    (`|SpawnActorFromClass` "/Game/Environment/Blueprints/MovingCar.MovingCar_C" (`self.GetTransform`) "AlwaysSpawn" "OverrideRootScale" null null)
    (set `self.TimeProgress` 0.0)
    (set `self.TimePeriod` (`KismetMathLibrary.RandomFloatInRange` 3.0 7.0))))

(fn `UserConstructionScript`)