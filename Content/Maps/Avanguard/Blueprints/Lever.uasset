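; Interactive lever for the Avanguard map that opens and closes every AvanguardDoor actor in the level.
; DoAction plays or reverses a timeline based on the SwitchedOn state, ignoring calls while it is running, to rotate the arm between closed and open rotations.
; When the swing finishes, it plays an attached sound, flips the state and sends OpenMessage or CloseMessage to all those doors.
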(event `self.DoAction`
  (params (Caller :type "Actor Object Reference"))
  (if (`TimelineComponent.IsPlaying` (`self.ActionTL`))
    _
    (elif (`self.SwitchedOn`)
      (bind (_direction _progress) (`Timeline|ActionTL` :!via `Reverse` :!label _label)
        (:`Update`
          (`SceneComponent.K2_SetRelativeRotation` (`self.Lever_Arm`) (`KismetMathLibrary.RLerp` (`self.CloseRot`) (`self.OpenRot`) _progress true) false false))
        (:`Finished`
          (`GameplayStatics.SpawnSoundAttached` "/Game/Sounds/Interact/b_rmz.b_rmz" (`self.Lever_Lever`) "None" (0.0 0.0 0.0) (struct) "KeepRelativeOffset" false 1.0 1.0 0.0 null null)
          (bind _output_get (set `self.SwitchedOn` (not (`self.SwitchedOn`))))
          (bind _outactors (`GameplayStatics.GetAllActorsOfClass` "/Game/Maps/Avanguard/Blueprints/AvanguardDoor.AvanguardDoor_C"))
          (for _array_element _outactors
            (if _output_get
              (message `/Game/Maps/Avanguard/Blueprints/AvanguardDoorInterface.Open` _array_element)
              (else
                (message `/Game/Maps/Avanguard/Blueprints/AvanguardDoorInterface.Close` _array_element))))))
      (else
        (goto _label)))))

(fn `UserConstructionScript`)